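; SpawningController_BP populates the level with monsters at randomly chosen spawn points when play begins.
; On BeginPlay it gathers all Spawner_BP actors, shuffles them and loops from index zero to MonsterRate, so each pick is a different spawner.
; Each picked spawner's MonsterType selects the Moth, Theri or Cere Blueprint, spawned at that spawner's location and rotation with collision adjustment that always spawns.
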(event EventBeginPlay
  (bind _outactors (Actor|GetAllActorsOfClass "/Game/Resource/Blueprints/Spawner_BP.Spawner_BP_C"))
  (bind _output_get (Variables|Default|SetSpawners _outactors))
  (Utilities|Array|Shuffle _output_get)
  (for _index (range 0 (Variables|Default|GetMonster%20Rate))
    (Game|SpawnActorfromClass (Utilities|Select :Index (Variables|/Game/Resource/Blueprints/Spawner_BP.Spawner_BP_C|GetMonster%20Type (Utilities|Array|Get(acopy) (Variables|Default|GetSpawners) _index)) :NewEnumerator0 "/Game/Resource/Character/Monster1/Moth_BP.Moth_BP_C" :NewEnumerator1 "/Game/Resource/Character/Theri/Theri_BP.Theri_BP_C" :NewEnumerator2 "/Game/Resource/Character/Cere/Cere_BP.Cere_BP_C") (Math|Transform|MakeTransform (Transformation|GetActorLocation (Utilities|Array|Get(acopy) (Variables|Default|GetSpawners) _index)) (Transformation|GetActorRotation (Utilities|Array|Get(acopy) (Variables|Default|GetSpawners) _index)) "1,1,1") "AdjustIfPossibleButAlwaysSpawn" 0)))

(fn ConstructionScript)