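; Checkpoint station that the player activates once to light it and record progress in the Gamedata game instance.
; Interaction stores the candle count, a respawn transform from PlayerBox and its display name, then shows the Loading widget.
; Lighting plays a sound and a timeline that brightens the point light from blue to orange.
; On BeginPlay, the checkpoint matching the saved name registers itself in Gamedata and relights after a delay.
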(event Custom|Lit%20Station
  (bind _pointlight (Variables|Default|GetPointLight))
  ;[1 0.2344 0] Effects
  (Variables|Default|Setactivated true)
  (Audio|SpawnSoundatLocation "/Game/Resource/Sound/Elevator_Button.Elevator_Button" (Transformation|GetActorLocation) "0, 0, 0" 0.3 1.0 0.0 "/Game/Resource/Sound/NewSoundAttenuation.NewSoundAttenuation" 0)
  (bind _alpha (Timeline|Lit PlayFromStart)
    (:Update
      (Rendering|Components|Light|SetIntensity _pointlight (Math|Float|Lerp 5e+02 4e+03 _alpha))
      (Rendering|Components|Light|SetLightColor _pointlight (Math|Color|Lerp(LinearColor) "(R=0.000000,G=0.439657,B=1.000000,A=1.000000)" "(R=1.000000,G=0.558341,B=0.132868,A=1.000000)" _alpha) true))))

(event EventBeginPlay
  ;[1 0.5156 0] Initial
  (bind _asgamedata (Utilities|Casting|CastToGamedata (Game|GetGameInstance)))
  (if (Utilities|Enum|Equal(Enum) (Variables|/Game/StoryAdvTemplate/Blueprints/Gamedata.Gamedata_C|GetCheckpoint_name _asgamedata) (Utilities|GetDisplayName self))
    (Variables|/Game/StoryAdvTemplate/Blueprints/Gamedata.Gamedata_C|SetCheckpoint_ref _asgamedata self)
    (Utilities|FlowControl|Delay 4.7)
    (CallFunction|LitStation)))

(event EventInteraction
  (bind _pointlight (Variables|Default|GetPointLight))
  (if (not (Variables|Default|Getactivated))
    (Utilities|FlowControl|Sequence
      (:then_0
        ;[1 0.2344 0] Effects
        (Variables|Default|Setactivated true)
        (Audio|SpawnSoundatLocation "/Game/Resource/Sound/Elevator_Button.Elevator_Button" (Transformation|GetActorLocation) "0, 0, 0" 0.3 1.0 0.0 "/Game/Resource/Sound/NewSoundAttenuation.NewSoundAttenuation" 0)
        (bind _alpha (Timeline|Lit PlayFromStart)
          (:Update
            (Rendering|Components|Light|SetIntensity _pointlight (Math|Float|Lerp 5e+02 4e+03 _alpha))
            (Rendering|Components|Light|SetLightColor _pointlight (Math|Color|Lerp(LinearColor) "(R=0.000000,G=0.439657,B=1.000000,A=1.000000)" "(R=1.000000,G=0.558341,B=0.132868,A=1.000000)" _alpha) true))))
      (:then_1
        ;[1 0.4453 0] Save
        (bind _asgamedata (Utilities|Casting|CastToGamedata (Game|GetGameInstance)))
        (bind _asbp_first_person_character (Utilities|Casting|CastToBP_FirstPersonCharacter (Game|Player|GetPlayerPawn 0)))
        (Variables|/Game/StoryAdvTemplate/Blueprints/Gamedata.Gamedata_C|SetCandle%20Number _asgamedata (Variables|/Game/StoryAdvTemplate/Blueprints/BP_FirstPersonCharacter.BP_FirstPersonCharacter_C|GetCandleNum _asbp_first_person_character))
        (Variables|/Game/StoryAdvTemplate/Blueprints/Gamedata.Gamedata_C|SetPlayer%20Transform _asgamedata (Math|Transform|MakeTransform (Transformation|GetWorldLocation (Variables|Default|GetPlayer%20Box)) (Transformation|GetActorRotation)))
        (Variables|/Game/StoryAdvTemplate/Blueprints/Gamedata.Gamedata_C|SetCheckpoint_name _asgamedata (Utilities|GetDisplayName self))
        ;[0 1 0.25] Saved Widget
        (bind _returnvalue (UserInterface|CreateWidget "/Game/Resource/UMG/Loading.Loading_C"))
        (UserInterface|Viewport|AddtoViewport _returnvalue 0)))))

(fn ConstructionScript
  (|CallParentFunction))