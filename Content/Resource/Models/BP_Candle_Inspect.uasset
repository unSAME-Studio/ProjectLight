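; BP_Candle_Inspect is a candle object that adds to the player's candle count when it is destroyed.
; On Destroyed, it casts the player pawn to BP_FirstPersonCharacter and increments CandleNum, with no check on what caused the destruction.
; The construction script runs the parent's, then applies the StaticMesh variable to the Object component.
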(event EventBeginPlay
  (|CallParentFunction) ; This node is disabled and will not be called.\nDrag off pins to build functionality.
)

(event Collision|EventActorBeginOverlap
  (params (OtherActor :type Actor%20Object%20Reference)))

(event EventTick
  (params (DeltaSeconds :type Float%20%28single-precision%29)))

(event EventDestroyed
  (bind _asbp_first_person_character (Utilities|Casting|CastToBP_FirstPersonCharacter (Game|Player|GetPlayerPawn 0)))
  (Math|Integer|IncrementInt (Variables|/Game/StoryAdvTemplate/Blueprints/BP_FirstPersonCharacter.BP_FirstPersonCharacter_C|GetCandleNum _asbp_first_person_character)))

(fn ConstructionScript
  (|CallParentFunction)
  (Components|StaticMesh|SetStaticMesh (Variables|Default|GetObject) (Variables|Default|GetStaticMesh)))