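; Level-exit elevator actor that descends and loads the next level, or serves as an arrival elevator when Arrives is set.
; Arrival elevators only play a pre-game door-closing animation, while departing ones flicker their spotlight's intensity and color via a Timeline.
; A one-shot Activate closes the door with sound and camera shake, then lowers the actor on a looping timer.
; After TimeBeforeTransport, it plays a Level Sequence and opens NextLevel when that ends.
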(event Custom|Move%20Elevator
  ;[1 0 0.6328] Elevator Move
  (Transformation|SetActorLocation (+ (Transformation|GetActorLocation) "0, 0,-0.900000") false false))

(event Custom|Activate
  (bind _level_sequence (Variables|Default|GetLevel%20Sequence))
  (bind _sequenceplayer (Variables|/Script/LevelSequence.LevelSequenceActor|GetSequencePlayer _level_sequence))
  ;[0.2422 1 0] Activate
  (if (not (Variables|Default|GetArrives?))
    (Utilities|FlowControl|DoOnce false
      (:Completed
        (Audio|SpawnSoundatLocation "/Game/Resource/Sound/Elevator_Close.Elevator_Close" (Transformation|GetActorLocation) "0, 0, 0" 1.0 1.0 0.0 "/Game/Resource/Sound/NewSoundAttenuation.NewSoundAttenuation" 0)
        (Utilities|FlowControl|Delay 1.0)
        (Components|Animation|PlayAnimation (Variables|Default|GetElevator_door) "/Game/Resource/Models/Elevator/Elevator_door_Anim_Bone_door_Door_Close.Elevator_door_Anim_Bone_door_Door_Close" false)
        (Camera|PlayWorldCameraShake "/Game/Resource/Models/Elevator/Elevator_Shake.Elevator_Shake_C" (Transformation|GetActorLocation) 0.0 1e+03 0.0)
        (Utilities|FlowControl|Delay 4.0)
        ;[1 0 0.6328] Elevator Move
        (Utilities|Time|SetTimerbyEvent (delegate Custom|Move%20Elevator) 0.01 true)
        (Audio|SpawnSoundAttached "/Game/Resource/Sound/Elevator_Running_Cue.Elevator_Running_Cue" (Variables|Default|GetElevator_lamp) "None" "0, 0, 0" "0, 0, 0" "SnapToTarget" false 1.0 1.0 0.0 "/Game/Resource/Sound/NewSoundAttenuation.NewSoundAttenuation" 0)
        ;[0 1 0.2734] Transporting
        (Utilities|FlowControl|Delay (Variables|Default|GetTime_before_transport))
        (Sequencer|Player|Play _sequenceplayer :!class /Script/MovieScene.MovieSceneSequencePlayer)
        (Utilities|FlowControl|Delay (Class|TimeManagementBlueprintLibrary|ToSeconds(QualifiedFrameTime) (Media|MediaPlayer|GetDuration _sequenceplayer)))
        (Game|OpenLevel(byName) (Variables|Default|GetNext%20Level))))))

(event EventBeginPlay
  ;[0 0.9531 1] If Arrive
  (if (Variables|Default|GetArrives?)
    (Components|Animation|PlayAnimation (Variables|Default|GetElevator_door) "/Game/Resource/Models/Elevator/Elevator_door_Anim_Bone_door_Door_Closebeforegame.Elevator_door_Anim_Bone_door_Door_Closebeforegame" false)
    (else
      ;[1 0 0.3047 0.5] Flicking light
      (bind (_direction _intensity _color) (Timeline|Timeline_0 PlayFromStart)
        (:Update
          (Utilities|FlowControl|Sequence
            (:then_0
              (Rendering|Components|Light|SetIntensity (Variables|Default|GetSpotLight) (* _intensity 2e+04)))
            (:then_1
              (Rendering|Components|Light|SetLightColor (Variables|Default|GetSpotLight) (Math|Color|Lerp(LinearColor) "(R=1.000000,G=0.560000,B=0.140000,A=1.000000)" "(R=0.796875,G=0.290629,B=0.105912,A=1.000000)" _color) true))))))))

(fn ConstructionScript)