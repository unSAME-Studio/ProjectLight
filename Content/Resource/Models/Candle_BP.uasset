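; Candle actor that burns down over time, flickering and shrinking as its wax melts, then goes out with smoke and sound before destroying itself.
; A looping timer drains Percentage to drive mesh scales and light intensity, while a timeline modulates flicker and color.
; A sphere matching the light radius registers the candle with Moth_BP.
; A second timer line-traces to the moth, computing Brightness from remaining wax and distance falloff, zero when blocked.
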(event OnComponentBeginOverlap(Sphere)
  (params (OverlappedComponent :type Primitive%20Component%20Object%20Reference) (OtherActor :type Actor%20Object%20Reference) (OtherComp :type Primitive%20Component%20Object%20Reference) (OtherBodyIndex :type Integer) (bFromSweep :type Boolean) (SweepResult :type Hit%20Result%20Structure%20%28by%20ref%29))
  ;[0.8281 1 0 0.5] Add Ref to moth
  (if (not (Variables|Default|Getdead?))
    (bind _asmoth_bp (Utilities|Casting|CastToMoth_BP OtherActor))
    (Utilities|Array|AddUnique (Variables|/Game/Resource/Character/Monster1/Moth_BP.Moth_BP_C|GetLights _asmoth_bp) self)
    (Variables|Default|SetMoth _asmoth_bp)))

(event OnComponentEndOverlap(Sphere)
  (params (OverlappedComponent :type Primitive%20Component%20Object%20Reference) (OtherActor :type Actor%20Object%20Reference) (OtherComp :type Primitive%20Component%20Object%20Reference) (OtherBodyIndex :type Integer))
  ;[0.8281 1 0 0.5] Add Ref to moth
  (if (not (Variables|Default|Getdead?))
    (bind _asmoth_bp (Utilities|Casting|CastToMoth_BP OtherActor))
    (Utilities|Array|RemoveItem (Variables|/Game/Resource/Character/Monster1/Moth_BP.Moth_BP_C|GetLights _asmoth_bp) self)
    (Variables|Default|SetMoth 0)))

(event Custom|Check%20Candle
  (bind _returnvalue (Transformation|GetActorLocation))
  (bind _moth (Variables|Default|GetMoth))
  ;[1 0.1875 0 0.5] Check Candle
  (bind _output_get (Variables|Default|SetPercentage (- (Variables|Default|GetPercentage) (Variables|Default|GetSpeed))))
  (if (<= _output_get 0.0)
    (Utilities|FlowControl|DoOnce false
      (:Completed
        (Variables|Default|Setdead? true)
        (Rendering|SetVisibility (Variables|Default|GetPointLight) false false)
        (Audio|SpawnSoundatLocation "/Game/Resource/Sound/Burnt.Burnt" _returnvalue "0, 0, 0" 1.0 1.0 0.0 "/Game/Resource/Sound/NewSoundAttenuation.NewSoundAttenuation" 0)
        (Effects|SpawnEmitteratLocation "/Game/Resource/SFX/Candle/P_Candlesmoke.P_Candlesmoke" _returnvalue)
        ;;[0 1 0.1328 0.5] Remove candle from the list if exist
        (Utilities|IsValid _moth
          (:Is%20Valid
            (Utilities|Array|RemoveItem (Variables|/Game/Resource/Character/Monster1/Moth_BP.Moth_BP_C|GetLights _moth) self))
          (:Is%20Not%20Valid
            _))
        (Utilities|FlowControl|Delay 1e+01)
        (Actor|DestroyActor)))
    (else
      (Transformation|SetRelativeScale3D (Variables|Default|GetCandle) (Math|Vector|MakeVector 0.1 0.1 (Math|Float|Lerp 0.009414 0.1 (/ (Variables|Default|GetPercentage) 1e+02))))
      (Transformation|SetRelativeScale3D (Variables|Default|GetCandle_Melt) (Math|Vector|Lerp(Vector) "0.100000,0.100000,0.100000" "0, 0, 0" (/ (Variables|Default|GetPercentage) 1e+02)))
      (Rendering|Components|Light|SetIntensity (Variables|Default|GetPointLight) (Math|Float|Lerp 1e+01 4e+03 (/ (Variables|Default|GetPercentage) 1e+02))))))

(event Custom|RaytraceTick
  (bind _pointlight (Variables|Default|GetPointLight))
  (bind _attenuationradius (Variables|/Script/Engine.LocalLightComponent|GetAttenuationRadius _pointlight))
  ;[0.4531 0 1 0.5] Ray Trace Tick
  (if (not (Variables|Default|Getdead?))
    (Utilities|IsValid (Variables|Default|GetMoth)
      (:Is%20Valid
        (bind _outhit (Collision|LineTraceByChannel (Transformation|GetWorldLocation (Variables|Default|GetPointLight)) (Transformation|GetActorLocation (Variables|Default|GetMoth)) "TraceTypeQuery2" false 0 "None"))
        (Utilities|Casting|CastToMoth_BP (.HitActor (Collision|BreakHitResult _outhit))
          (:then
            (Variables|Default|SetBrightness (* (/ (Variables|Default|GetPercentage) 5e+01) (|(pow((1-(pow((distance/radius),4))),2)) (Math|Float|Min(Float) (Transformation|GetDistanceTo (Variables|Default|GetMoth)) _attenuationradius) _attenuationradius))))
          (:CastFailed
            (Variables|Default|SetBrightness 0.0))))
      (:Is%20Not%20Valid
        (Variables|Default|SetBrightness 0.0)))))

(event EventBeginPlay
  ;[0 0.08594 1 0.5] P
  (Audio|SpawnSoundatLocation "/Game/Resource/Sound/Drop_Candle.Drop_Candle" (Transformation|GetActorLocation) "0, 0, 0" 1.0 1.0 0.0 "/Game/Resource/Sound/NewSoundAttenuation.NewSoundAttenuation" 0)
  (Utilities|Time|SetTimerbyFunctionName 0 "Check Candle" 0.1 true)
  (Utilities|Time|SetTimerbyFunctionName 0 "RaytraceTick" 0.1 true)
  ;[0.4062 1 0 0.5] Set Sphere Radius
  (Components|Sphere|SetSphereRadius (Variables|Default|GetSphere) (Variables|/Script/Engine.LocalLightComponent|GetAttenuationRadius (Variables|Default|GetPointLight)) true)
  ;[1 0 0.3047 0.5] Flicking light
  (bind (_direction _intensity _color) (Timeline|Timeline_0 Play)
    (:Update
      (Utilities|FlowControl|Sequence
        (:then_0
          (Rendering|Components|Light|SetIntensity (Variables|Default|GetPointLight) (* _intensity (Variables|/Script/Engine.LightComponentBase|GetIntensity (Variables|Default|GetPointLight)))))
        (:then_1
          (Rendering|Components|Light|SetLightColor (Variables|Default|GetPointLight) (Math|Color|Lerp(LinearColor) "(R=1.000000,G=0.560000,B=0.140000,A=1.000000)" "(R=0.796875,G=0.290629,B=0.105912,A=1.000000)" _color) true))))))

(fn ConstructionScript)