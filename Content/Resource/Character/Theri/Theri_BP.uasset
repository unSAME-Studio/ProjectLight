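; Theri is an enemy that notices the nearby player, turns to face them and dives at a lit candle to snuff it.
; A looping timer checks distance, triggering a one-time notice sound and yaw tracking, then line-traces at closer range.
; Seeing the player with the candle on triggers a one-shot montage and timeline lerp onto the player's position.
; On arrival it zeroes the candle value if still lit, then destroys itself regardless.
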(event Custom|Tick
  ;[0 0.7891 1] Tick
  (CallFunction|Trace4Player))

(event Custom|Notice%20Sound
  ;[1 0.4453 0] Notice Sound
  (Utilities|FlowControl|DoOnce false
    (:Completed
      (Audio|SpawnSoundatLocation "/Game/Resource/Sound/Theri_Notice.Theri_Notice" (Transformation|GetActorLocation) "0, 0, 0" 1.0 1.0 0.0 "/Game/Resource/Sound/NewSoundAttenuation.NewSoundAttenuation" 0))))

(event Custom|Fly
  ;[0.8984 1 0] Fly Toward Player
  (Utilities|FlowControl|DoOnce false
    (:Completed
      (Audio|SpawnSound2D "/Game/Resource/Sound/Theri_Fly_Cue.Theri_Fly_Cue" 0.6 1.0 0.0 0)
      (Animation|Montage|PlayMontage (Variables|Character|GetMesh) "/Game/Resource/Character/Theri/Monster2_Anim_Bone_Boi2_Notice_Montage.Monster2_Anim_Bone_Boi2_Notice_Montage"
        (:then
          (Utilities|FlowControl|Delay 0.4)
          (Variables|Default|SetInitial%20Location (Transformation|GetActorLocation))
          (bind _location (Timeline|Fly%20Toward PlayFromStart)
            (:Update
              (Transformation|SetActorLocation (Math|Vector|Lerp(Vector) (Variables|Default|GetInitial%20Location) (Transformation|GetActorLocation (Game|Player|GetPlayerPawn 0)) _location) false false))
            (:Finished
              (bind _asbp_first_person_character (Utilities|Casting|CastToBP_FirstPersonCharacter (Game|Player|GetPlayerPawn 0)))
              (if (Variables|/Game/StoryAdvTemplate/Blueprints/BP_FirstPersonCharacter.BP_FirstPersonCharacter_C|GetCandle%20On? _asbp_first_person_character)
                (Variables|/Game/StoryAdvTemplate/Blueprints/BP_FirstPersonCharacter.BP_FirstPersonCharacter_C|SetCandleValue _asbp_first_person_character 0.0)
                (Actor|DestroyActor)
                (else
                  (Actor|DestroyActor))))))))))

(event EventBeginPlay
  (Utilities|Time|SetTimerbyFunctionName 0 "Tick" 0.1 true)
  ;[1 0.3047 0 0.5] Set Player Ref
  (bind _asbp_first_person_character (Utilities|Casting|CastToBP_FirstPersonCharacter (Game|Player|GetPlayerPawn 0)))
  (Variables|Default|SetPlayer_Ref _asbp_first_person_character))

(event EventTick
  (params (DeltaSeconds :type Float%20%28single-precision%29))
  ;[0.4531 0 1] Face Player
  (if (Variables|Default|GetFacePlayer?)
    (Transformation|SetActorRotation (Math|Rotator|MakeRotator 0.0 0.0 (.yaw (Math|Interpolation|RInterpTo (Transformation|GetActorRotation) (Math|Rotator|FindLookatRotation (Transformation|GetActorLocation) (Transformation|GetActorLocation (Game|Player|GetPlayerPawn 0))) DeltaSeconds 2.0))))))

(fn ConstructionScript)

(fn Trace4Player
  (bind _player_ref (Variables|Default|GetPlayer_Ref))
  (bind _returnvalue (Transformation|GetDistanceTo _player_ref))
  (if (< _returnvalue 2.5e+03)
    (Variables|Default|SetNotice? true)
    (Variables|Default|SetFacePlayer? true)
    (CallFunction|NoticeSound)
    (if (< _returnvalue 1e+03)
      ;[0 1 0.2969] Line Trace for player
      (bind (_outhit _returnvalue_2) (Collision|LineTraceByChannel (Transformation|GetWorldLocation (Variables|Default|GetBox)) (Transformation|GetActorLocation (Variables|Default|GetPlayer_Ref)) "TraceTypeQuery2" false 0 "None"))
      (if _returnvalue_2
        (bind _asbp_first_person_character (Utilities|Casting|CastToBP_FirstPersonCharacter (.HitActor (Collision|BreakHitResult _outhit)))
          (:then
            (if (Variables|/Game/StoryAdvTemplate/Blueprints/BP_FirstPersonCharacter.BP_FirstPersonCharacter_C|GetCandle%20On? _asbp_first_person_character)
              (CallFunction|Fly)))
          (:CastFailed
            (Development|PrintString "Hit Walls" true true "(R=1.000000,G=0.685056,B=0.000000,A=1.000000)")))))
    (else
      (Variables|Default|SetNotice? false)
      (Variables|Default|SetFacePlayer? false))))