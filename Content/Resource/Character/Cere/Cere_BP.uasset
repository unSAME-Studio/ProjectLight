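; Cere is a flying suicide-bomber creature that wakes near the player, seeks the closest light and explodes beside it.
; A looping timer checks player distance and finds the nearest entry in Lights, driving movement input, while per-frame Tick smoothly turns it toward that target.
; Within blast range it raises fly speed, then after a delay sphere-traces to damage the player and zero candle percentages, and destroys itself.
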(event Custom|Tick
  ;[0 0.7891 1] Tick
  (CallFunction|CheckPlayerDistance)
  (CallFunction|CheckAllLightDistance))

(event Custom|Exploded
  (bind _returnvalue (Transformation|GetActorLocation))
  ;[0 1 1] Exploded
  (Utilities|FlowControl|DoOnce false
    (:Completed
      (Development|PrintString "EXPLODED!!!" true true "(R=1.000000,G=0.241172,B=0.000000,A=1.000000)")
      (Variables|Default|SetExplode true)
      (Utilities|FlowControl|Sequence
        (:then_0
          ;;[0.05469 0 1] Movement
          (Variables|/Script/Engine.CharacterMovementComponent|SetMaxFlySpeed (Variables|Character|GetCharacterMovement) 1.2e+03)
          (Pawn|Input|AddMovementInput (Transformation|GetActorForwardVector) 1.0 false))
        (:then_1
          (Utilities|FlowControl|Delay 1.0)
          (bind _outhits (Collision|MultiSphereTraceByChannel _returnvalue (+ _returnvalue "0, 0,50.000000") 2e+02 "TraceTypeQuery2" false 0 "ForDuration"))
          (for _array_element _outhits
            (bind _asbp_first_person_character (Utilities|Casting|CastToBP_FirstPersonCharacter (.HitActor (Collision|BreakHitResult _array_element)))
              (:then
                (Default|DealDamage _asbp_first_person_character 5e+01))
              (:CastFailed
                (bind _ascandle_bp (Utilities|Casting|CastToCandle_BP (.HitActor (Collision|BreakHitResult _array_element))))
                (Variables|/Game/Resource/Models/Candle_BP.Candle_BP_C|SetPercentage _ascandle_bp 0.0))))
          (Actor|DestroyActor))))))

(event EventBeginPlay
  (Utilities|Time|SetTimerbyFunctionName 0 "Tick" 0.1 true)
  ;[1 0.3047 0 0.5] Set Player Ref
  (bind _asbp_first_person_character (Utilities|Casting|CastToBP_FirstPersonCharacter (Game|Player|GetPlayerPawn 0)))
  (Variables|Default|SetPlayer_Ref _asbp_first_person_character))

(event EventTick
  (params (DeltaSeconds :type Float%20%28single-precision%29))
  (bind _curent_closest_light (Variables|Default|GetCurent%20Closest%20Light))
  ;[0.4531 0 1] Face Player
  (if (Variables|Default|GetAwake)
    (Transformation|SetActorRotation (Math|Interpolation|RInterpTo (Transformation|GetActorRotation) (Math|Rotator|FindLookatRotation (Transformation|GetActorLocation) (Transformation|GetActorLocation (select (Utilities|IsValid _curent_closest_light) _curent_closest_light (Game|Player|GetPlayerPawn 0)))) DeltaSeconds 2.0))))

(fn ConstructionScript)

(fn CheckAllLightDistance
  (bind _lights_distance (Variables|Default|GetLights_Distance))
  (bind (_indexofminvalue _minvalue) (Math|Float|MinOfFloatArray _lights_distance))
  (if (and (Variables|Default|GetAwake) (not (Variables|Default|GetExplode)))
    (for _array_element (Variables|Default|GetLights)
      (Utilities|Array|Add (Variables|Default|GetLights_Distance) (Transformation|GetDistanceTo _array_element self)))
    (bind _output_get (Variables|Default|SetCurent%20Closest%20Light (Utilities|Array|Get(acopy) (Variables|Default|GetLights) _indexofminvalue)))
    (bind _output_get_2 (Variables|Default|SetCurent%20Light%20Distance _minvalue))
    (Development|PrintString (Utilities|GetDisplayName _output_get) true true "(R=0.000000,G=0.826424,B=1.000000,A=1.000000)")
    (Development|PrintString (Utilities|String|ToString(Float) _output_get_2) true true "(R=0.134855,G=1.000000,B=0.000000,A=1.000000)")
    (Utilities|Array|Clear (Variables|Default|GetLights_Distance))
    (CallFunction|Movement)))

(fn CheckPlayerDistance
  (if (not (Variables|Default|GetExplode))
    (if (and (< (Transformation|GetDistanceTo (Variables|Default|GetPlayer_Ref)) 2e+03) (Utilities|IsValid (Utilities|Array|Get(acopy) (Variables|Default|GetLights))))
      (Variables|Default|SetAwake true)
      (else
        (Variables|Default|SetAwake false)))))

(fn Movement
  (if (> (Variables|Default|GetCurent%20Light%20Distance) 2.5e+02)
    (Pawn|Input|AddMovementInput (Transformation|GetActorForwardVector) 1.0 false)
    (else
      (CallFunction|Exploded))))