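; Gamedata holds checkpoint state for the first-person player and handles respawning through its RevivePlayer event.
; The event clears the Revived flag, restores the stored candle count to the character and moves it to the saved player transform.
; It then spawns an actor at the checkpoint's candle spawn place and re-enables player input after a fixed delay.
; A DisableInput call is present but never runs.
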(event Custom|Revive%20Player
  (bind _player_transform (Variables|Default|GetPlayer%20Transform))
  (bind _checkpoint_ref (Variables|Default|GetCheckpoint_ref))
  (bind _candle_spawn_place (Variables|/Game/Resource/Models/Checkpoint/Checkpoint_BP.Checkpoint_BP_C|GetCandle%20Spawn%20Place _checkpoint_ref))
  (bind _returnvalue (Transformation|GetWorldTransform _candle_spawn_place))
  ;[0.5937 1 0] Revive Player
  (Variables|Default|SetRevived? false)
  (bind _asbp_first_person_character (Utilities|Casting|CastToBP_FirstPersonCharacter (Game|Player|GetPlayerPawn 0)))
  (Variables|Default|SetPlayer_Ref _asbp_first_person_character)
  (Variables|/Game/StoryAdvTemplate/Blueprints/BP_FirstPersonCharacter.BP_FirstPersonCharacter_C|SetCandleNum (Variables|Default|GetPlayer_Ref) (Variables|Default|GetCandle%20Number))
  (Transformation|SetActorLocationAndRotation (Variables|Default|GetPlayer_Ref) (.location _player_transform) (.rotation _player_transform))
  (Game|SpawnActorfromClass "/Game/Resource/Models/Candle_Object.Candle_Object_C" (Math|Transform|MakeTransform (.location _returnvalue) (.rotation _returnvalue) "1,1,1") "AlwaysSpawn" 0 0)
  (Utilities|FlowControl|Delay 4.7)
  (Input|EnableInput (Variables|Default|GetPlayer_Ref) (Game|GetPlayerController 0)))